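; BP_Enemy is an enemy Blueprint that shows its health on a widget component.
; On BeginPlay it casts the EnemyHealth component's widget to BP_Enemy_Health and caches the reference.
; Every Tick it pushes Health, divided by a fixed maximum of 100, into that widget's progress bar.
; Leftover animation and movement nodes are unconnected, and nothing here changes Health.
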(event `self.ReceiveBeginPlay`
  (bind _asbp_enemy_health (cast `/Game/Blueprints/UI/BP_Enemy_Health` (`WidgetComponent.GetUserWidgetObject` (`self.Enemy Health`))))
  (set `self.BP Enemy Health REF` _asbp_enemy_health))

(event `self.ReceiveTick`
  (params (DeltaSeconds :type "Float (single-precision)"))
  (`ProgressBar.SetPercent` (`/Game/Blueprints/UI/BP_Enemy_Health.HealthProgress` (`self.BP Enemy Health REF`)) (/ (`self.Health`) 100.0)))

(fn `UserConstructionScript`)